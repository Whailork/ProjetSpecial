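; BP_FlightRaceTrialGameMode is the game mode for the Flight Race trial, setting up its sublevel and trial time HUD.
; BeginPlay streams in the trial sublevel without blocking and, on authority, adds a UW_TrialTime widget to each local player's screen.
; PostLogin calls the parent handler, then also creates that widget for each player who logs in.
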(event `self.ReceiveBeginPlay`
  (`GameplayStatics.LoadStreamLevelBySoftObjectPtr` "/Game/Levels/Trials/SubLvl_FlightRaceTrial.SubLvl_FlightRaceTrial" true)
  (if (`self.HasAuthority`)
    (for _index (range (`GameplayStatics.GetNumLocalPlayerControllers`))
      (bind _returnvalue (`GameplayStatics.GetPlayerController` _index))
      (`/Engine/EditorBlueprintResources/StandardMacros.IsValid` _returnvalue
        (:`Is Valid`
          (bind _returnvalue_2 (`|CreateWidget` "/Game/HUD/UW_TrialTime.UW_TrialTime_C" _returnvalue))
          (`UserWidget.AddToPlayerScreen` _returnvalue_2 0))))))

(event `self.K2_PostLogin`
  (params (NewPlayer :type "PlayerController Object Reference"))
  (`parent.K2_PostLogin` NewPlayer)
  (bind _returnvalue (`|CreateWidget` "/Game/HUD/UW_TrialTime.UW_TrialTime_C" NewPlayer))
  (`UserWidget.AddToPlayerScreen` _returnvalue 0))

(fn `UserConstructionScript`)