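; Starting gate actor for race trials that begins the trial when a player passes through it.
; It fixes its gate number at zero in both the construction script and BeginPlay.
; On overlap with a pawn possessed by the race trial player controller, it tells that controller the trial has started and gate zero is reached.
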(event `self.ReceiveBeginPlay`
  (`parent.ReceiveBeginPlay`)
  (set `self.GateNumber` 0))

(event `self.ReceiveActorBeginOverlap`
  (params (OtherActor :type "Actor Object Reference"))
  (`parent.ReceiveActorBeginOverlap` OtherActor)
  (bind _aspawn (cast `Pawn` OtherActor))
  (bind _asbp_race_trial_player_controller (cast `/Game/Blueprints/Trials/BP_RaceTrialPlayerController` (`Pawn.GetController` _aspawn)))
  (`TrialPlayerController.TrialStarted` _asbp_race_trial_player_controller)
  (`RaceTrialPlayerController.GateReached` _asbp_race_trial_player_controller 0))

(fn `UserConstructionScript`
  (`parent.UserConstructionScript`)
  (set `self.GateNumber` 0))