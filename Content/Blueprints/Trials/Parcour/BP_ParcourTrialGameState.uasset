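; Game state for the parkour trial that ends a player's trial when their character touches something other than a parkour platform.
; On BeginPlay it binds a handler to the OnActorHit event of every ProjetSpecialCharacter already in the level.
; On a hit with a non-ParcoursPlatform actor, the handler calls TrialEnded(true) on the TrialPlayerController if the trial start time is set and the character is not falling.
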(event `self.ReceiveBeginPlay`
  (bind _outactors (`GameplayStatics.GetAllActorsOfClass` "/Script/ProjetSpecial.ProjetSpecialCharacter"))
  (for _array_element _outactors
    (add `Actor.OnActorHit` _array_element (delegate `CustomEvent`))))

(event `CustomEvent`
  (params (SelfActor :type "Actor Object Reference") (OtherActor :type "Actor Object Reference") (NormalImpulse :type "Vector Structure") (Hit :type "HitResult Structure (by ref)"))
  (bind _ascharacter (cast `Character` SelfActor))
  (bind _astrial_player_controller (cast `TrialPlayerController` (`Pawn.GetController` _ascharacter)))
  (cast `/Game/Blueprints/Trials/Parcour/ParcoursPlatform` OtherActor
    (:`CastFailed`
      (if (and (!= (`TrialPlayerController.TrialStartTime` _astrial_player_controller) 0.0) (not (`NavMovementComponent.IsFalling` (`Character.CharacterMovement` _ascharacter))))
        (`TrialPlayerController.TrialEnded` _astrial_player_controller true)))))

(fn `UserConstructionScript`)