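; Finish gate actor for race trials that ends the trial when the player crosses it.
; On actor overlap, it casts the other actor to a Pawn and that pawn's controller to a TrialPlayerController, then calls TrialEnded on the controller.
; Overlaps from anything else are ignored, and BeginPlay, Tick and the construction script add no logic.
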(event `self.ReceiveActorBeginOverlap`
  (params (OtherActor :type "Actor Object Reference"))
  (`parent.ReceiveActorBeginOverlap` OtherActor)
  (bind _aspawn (cast `Pawn` OtherActor))
  (bind _astrial_player_controller (cast `TrialPlayerController` (`Pawn.GetController` _aspawn)))
  (`TrialPlayerController.TrialEnded` _astrial_player_controller))

(fn `UserConstructionScript`
  (`parent.UserConstructionScript`))