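; BP_FoodPickup is a food pickup actor that extends a parent pickup, shows its type through a widget and fades out when despawning.
; SetupValues runs the parent setup, passes Type to the UW_FoodPickup widget, then launches BoxCollision with a random impulse in an upward cone.
; Once StartDespawnAnim is set, Tick plays a timeline that fades the widget's tint alpha and destroys the actor on finish.
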(event `self.SetupValues`
  (params (type :type "EFoodType Enum" :default "No"))
  (`parent.SetupValues` type)
  (bind _asuw_food_pickup (cast `/Game/HUD/UW_FoodPickup` (`WidgetComponent.GetWidget` (`self.AppearanceWidget`))))
  (set `/Game/HUD/UW_FoodPickup.Type` type _asuw_food_pickup)
  (`PrimitiveComponent.AddImpulse` (`self.BoxCollision`) (* (`KismetMathLibrary.RandomUnitVectorInConeInDegrees` (0.0 0.0 1.0) 50.0) 16000.0) "None" false))

(event `self.ReceiveTick`
  (params (DeltaSeconds :type "Float (single-precision)"))
  (if (`self.StartDespawnAnim`)
    (bind (_direction _newtrack_0) (`Timeline|Timeline` :`NewTime` DeltaSeconds)
      (:`Update`
        (`WidgetComponent.SetTintColorAndOpacity` (`self.AppearanceWidget`) (make `LinearColor` 1.0 1.0 1.0 _newtrack_0)))
      (:`Finished`
        (`self.K2_DestroyActor`)))))

(fn `UserConstructionScript`)