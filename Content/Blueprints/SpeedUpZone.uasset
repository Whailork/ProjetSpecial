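; SpeedUpZone is a trigger actor that boosts the flying speed of actors entering it.
; On overlap, with GlidingOnly set, it finds the actor's FlyingMovementComponent and, if gliding, adds SpeedUpStrength to CurrentFlyingSpeed, capped at MaxSpeed.
; The boost is a one-time addition per overlap.
; Without GlidingOnly, it only casts to ProjetSpecialCharacter and applies no effect.
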(event `self.ReceiveActorBeginOverlap`
  (params (OtherActor :type "Actor Object Reference"))
  (bind _returnvalue (`self.GetComponentByClass` OtherActor "/Script/ProjetSpecial.FlyingMovementComponent"))
  (if (`self.bGlidingOnly`)
    (`/Engine/EditorBlueprintResources/StandardMacros.IsValid` _returnvalue
      (:`Is Valid`
        (if (`FlyingMovementComponent.bIsGliding` _returnvalue)
          (set `FlyingMovementComponent.currentFlyingSpeed` (`KismetMathLibrary.FMin` (+ (`FlyingMovementComponent.currentFlyingSpeed` _returnvalue) (`self.SpeedUpStrength`)) (`self.MaxSpeed`)) _returnvalue))))
    (else
      (cast `ProjetSpecialCharacter` OtherActor))))

(fn `UserConstructionScript`)