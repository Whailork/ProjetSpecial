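; Breakable power-up jar that uses a Chaos Geometry Collection and drops power-ups when destroyed.
; Early hits from the player or a fireball trigger that source's AttackMasterField, counting up until a later hit starts the explosion.
; The final hit spawns a master field and disables box collision, then Tick applies fields and disables clustering for a few frames.
; PowerUpManager then generates and spawns drops around the jar, which destroys itself after a delay.
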(event `self.OnHittableObjectHit`
  (params (damage :type "Float (single-precision)") (Source :type "Actor Object Reference") (Hit :type "HitResult Structure"))
  (if (< (`self.AttackCount`) 3)
    (bind _asbp_third_person_character (cast `/Game/ThirdPerson/Blueprints/BP_ThirdPersonCharacter` Source)
      (:`then`
        (bind _asbp_attack_master_field (cast `/Game/Blueprints/BP_AttackMasterField` (`ChildActorComponent.ChildActor` (`/Game/ThirdPerson/Blueprints/BP_ThirdPersonCharacter.AttackMasterField` _asbp_third_person_character))))
        (`/Engine/EditorResources/FieldNodes/FS_MasterField.CE_Trigger` _asbp_attack_master_field))
      (:`CastFailed`
        (bind _asbp_fireball (cast `/Game/Blueprints/BP_Fireball` Source))
        (bind _asbp_attack_master_field_2 (cast `/Game/Blueprints/BP_AttackMasterField` (`ChildActorComponent.ChildActor` (`/Game/Blueprints/BP_Fireball.AttackMasterField` _asbp_fireball))))
        (`/Engine/EditorResources/FieldNodes/FS_MasterField.CE_Trigger` _asbp_attack_master_field_2)))
    (`/Engine/EditorBlueprintResources/StandardMacros.IncrementInt` (`self.AttackCount`))
    (else
      (set `self.bExplode` true)
      (bind _returnvalue (`|SpawnActorFromClass` "/Game/Blueprints/BP_AttackMasterField.BP_AttackMasterField_C" (`KismetMathLibrary.MakeTransform` (`self.K2_GetActorLocation`) (struct) (1.0 1.0 3.0)) "Undefined" "MultiplyWithRoot" null null))
      (bind _output_get (set `self.MasterField` _returnvalue))
      (set `/Engine/EditorResources/FieldNodes/FS_MasterField.ActivationType` "NewEnumerator2" _output_get)
      (`PrimitiveComponent.SetCollisionEnabled` (`self.BoxVolumeCol`) "NoCollision"))))

(event `self.ReceiveTick`
  (params (DeltaSeconds :type "Float (single-precision)"))
  (bind _returnvalue (`self.K2_GetActorLocation`))
  (bind _returnvalue_2 (subsystem `PowerUpManager`))
  (bind _destroycount (`self.DestroyCount`))
  (if (`self.bExplode`)
    (`GeometryCollectionComponent.ApplyKinematicField` (`self.GeometryCollection`) 500.0 _returnvalue)
    (`FieldSystemComponent.ApplyStayDynamicField` (`self.FieldSystemComponent`) false _returnvalue 500.0)
    (set `GeometryCollectionComponent.EnableClustering` false (`self.GeometryCollection`))
    (if (> _destroycount 4)
      (set `self.bExplode` false)
      (`self.K2_DestroyActor` (`self.MasterField`))
      (bind _returnvalue_3 (`PowerUpManager.GeneratePowerUpDrops` _returnvalue_2))
      (`PowerUpManager.SpawnPowerUps` _returnvalue_2 _returnvalue_3 (`self.K2_GetActorLocation`))
      (`KismetSystemLibrary.Delay` 6.0)
      (`self.K2_DestroyActor`)
      (else
        (`/Engine/EditorBlueprintResources/StandardMacros.IncrementInt` _destroycount)))))

(fn `UserConstructionScript`
  (bind _initializationfields (`GeometryCollectionComponent.InitializationFields` (`self.GeometryCollection`)))
  (`parent.UserConstructionScript`)
  (`KismetArrayLibrary.Array_Clear` _initializationfields)
  (`KismetArrayLibrary.Array_Add` _initializationfields self))