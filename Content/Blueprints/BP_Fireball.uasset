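; BP_Fireball is a fireball attack actor that damages a HitableActor it hits, using its spawner character's Strength.
; Timers set at BeginPlay make its sphere block WorldDynamic after a short delay and later despawn it along with its child field actor.
; A successful hit also fires CETrigger on the child BP_AttackMasterField, then destroys both after a brief delay.
; Hits on other actors are ignored, leaving cleanup to the despawn timer.
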(event `self.ReceiveBeginPlay`
  (`KismetSystemLibrary.K2_SetTimerDelegate` (delegate `Activate dynamic collisions`) 0.4)
  (`KismetSystemLibrary.K2_SetTimerDelegate` (delegate `Despawn`) 3.0))

(event `Despawn`
  (bind _childactor (`ChildActorComponent.ChildActor` (`self.AttackMasterField`)))
  (`/Engine/EditorBlueprintResources/StandardMacros.IsValid` _childactor
    (:`Is Valid`
      (`self.K2_DestroyActor` _childactor))
    (:`Is Not Valid`
      _))
  (`self.K2_DestroyActor`))

(event `Activate dynamic collisions`
  (`PrimitiveComponent.SetCollisionResponseToChannel` (`self.SphereComponent`) "ECC_WorldDynamic" "ECR_Block"))

(event `self.SphereComponent.OnComponentHit`
  (params (HitComponent :type "PrimitiveComponent Object Reference") (OtherActor :type "Actor Object Reference") (OtherComp :type "PrimitiveComponent Object Reference") (NormalImpulse :type "Vector Structure") (Hit :type "HitResult Structure (by ref)"))
  (bind _ashitable_actor (cast `HitableActor` OtherActor))
  (`HitableActor.OnHittableObjectHit` _ashitable_actor (`ProjetSpecialCharacter.Strength` (`self.SpawnerCharacter`)) self Hit)
  (bind _asbp_attack_master_field (cast `/Game/Blueprints/BP_AttackMasterField` (`ChildActorComponent.ChildActor` (`self.AttackMasterField`))))
  (`/Engine/EditorResources/FieldNodes/FS_MasterField.CE_Trigger` _asbp_attack_master_field)
  (`KismetSystemLibrary.Delay` 0.08)
  (`/Engine/EditorBlueprintResources/StandardMacros.IsValid` _asbp_attack_master_field
    (:`Is Valid`
      (`self.K2_DestroyActor` _asbp_attack_master_field))
    (:`Is Not Valid`
      _))
  (`self.K2_DestroyActor`))

(fn `UserConstructionScript`)