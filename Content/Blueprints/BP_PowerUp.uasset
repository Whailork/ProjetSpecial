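; BP_PowerUp is a power-up actor that pops into the world with a type and a positive or negative flag.
; SetupTypeValues calls the parent, passes both values to the UW_PowerUp in its AppearanceWidget, then launches BoxCollision with a random impulse inside an upward cone.
; Tick polls StartDespawnAnim and, while it is set, plays a timeline that animates the widget's opacity and destroys the actor when finished.
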(event `self.SetupTypeValues`
  (params (typeValue :type "EPowerUpType Enum" :default "Speed") (negativeValue :type Boolean))
  (`parent.SetupTypeValues` typeValue negativeValue)
  (bind _asuw_power_up (cast `/Game/HUD/UW_PowerUp` (`WidgetComponent.GetWidget` (`self.AppearanceWidget`))))
  (set `/Game/HUD/UW_PowerUp.Type` typeValue _asuw_power_up)
  (set `/Game/HUD/UW_PowerUp.IsNegative` negativeValue _asuw_power_up)
  (`PrimitiveComponent.AddImpulse` (`self.BoxCollision`) (* (`KismetMathLibrary.RandomUnitVectorInConeInDegrees` (0.0 0.0 1.0) 45.0) 15000.0) "None" false))

(event `self.ReceiveBeginPlay`)

(event `self.ReceiveTick`
  (params (DeltaSeconds :type "Float (single-precision)"))
  (if (`self.StartDespawnAnim`)
    (bind (_direction _newtrack_0) (`Timeline|Timeline` :`NewTime` DeltaSeconds)
      (:`Update`
        (`WidgetComponent.SetTintColorAndOpacity` (`self.AppearanceWidget`) (make `LinearColor` 1.0 1.0 1.0 _newtrack_0)))
      (:`Finished`
        (`self.K2_DestroyActor`)))))

(fn `UserConstructionScript`)